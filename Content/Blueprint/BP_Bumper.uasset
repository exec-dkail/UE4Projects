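; BP_Bumper is a pinball-style bumper actor that knocks a BP_Ball away when the ball overlaps it.
; The Bump event applies a velocity-change impulse along the direction from bumper to ball and plays an attached hit sound.
; A timeline then drives the mechanism's vertical offset, the light intensity and an emissive parameter on a dynamic material created in the construction script.
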(event `self.ReceiveActorBeginOverlap`
  (params (OtherActor :type "Actor Object Reference"))
  (bind _asbp_ball (cast `/Game/Blueprint/BP_Ball` OtherActor))
  (`self.Bump` _asbp_ball))

(event `Bump`
  (params (Ball :type "/Game/Blueprint/BP_Ball Object Reference"))
  (`PrimitiveComponent.AddImpulse` (`/Game/Blueprint/BP_Ball.Ball` Ball) (* (`KismetMathLibrary.GetDirectionUnitVector` (`self.K2_GetActorLocation`) (`self.K2_GetActorLocation` Ball)) 2500.0) "None" true)
  (`GameplayStatics.SpawnSoundAttached` "/Game/Assets/Sounds/BumperHit.BumperHit" (`self.BumperBase`))
  (bind (_direction _newtrack_0) (`Timeline|BumpActivator` :!via `PlayFromStart`)
    (:`Update`
      (`SceneComponent.K2_SetRelativeLocation` (`self.BumperMech`) (`KismetMathLibrary.VLerp` (0.0 0.0 0.0) (0.0 0.0 -70.0) _newtrack_0) false false)
      (`LightComponent.SetIntensity` (`self.BumperLight`) (`KismetMathLibrary.Lerp` 0.0 15000.0 _newtrack_0))
      (`MaterialInstanceDynamic.SetScalarParameterValue` (`self.Bumper_MID`) "EmmisiveMultiplier" (`KismetMathLibrary.Lerp` 0.0 25.0 _newtrack_0)))))

(fn `UserConstructionScript`
  (bind _returnvalue (`PrimitiveComponent.CreateDynamicMaterialInstance` (`self.BumperBase`) 1 null))
  (set `self.Bumper_MID` _returnvalue))